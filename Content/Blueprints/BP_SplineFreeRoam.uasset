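; BP_SplineFreeRoam moves player pawn 0 along the WayToFollow spline while free roam is switched on.
; StartFreeRoam and StopFreeRoam toggle a flag that Tick checks before calling MoveToNextPoint.
; Each step teleports the pawn to a TInterpTo blend toward the current spline point's world transform, following points rather than the curve between them.
; Within a small distance it advances to the next point, looping back to the first after the last.
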(event Custom|StartFreeRoam
  (Variables|Default|SetFreeRoaming true))

(event Custom|MoveToNextPoint
  (bind _returnvalue (Game|Player|GetPlayerPawn 0))
  (bind _returnvalue_2 (Transformation|GetActorTransform _returnvalue))
  (Transformation|SetActorTransform (Game|Player|GetPlayerPawn 0) (Class|KismetMathLibrary|TInterpto _returnvalue_2 (Spline|GetTransformatSplinePoint (Variables|Default|GetWayToFollow) (Variables|Default|GetCurrentPoint) "World" false) (Variables|Default|GetDeltaT) (Variables|Default|GetSpeed)) false true)
  (if (< (Math|Vector|Distance(Vector) (.Location (Math|Transform|BreakTransform _returnvalue_2)) (.Location (Math|Transform|BreakTransform (Spline|GetTransformatSplinePoint (Variables|Default|GetWayToFollow) (Variables|Default|GetCurrentPoint) "World" false)))) 0.2)
    (bind _result (Math|Integer|IncrementInt (Variables|Default|GetCurrentPoint))
      (:%20%20
        (if (>= _result (Spline|GetNumberOfSplinePoints (Variables|Default|GetWayToFollow)))
          (Variables|Default|SetCurrentPoint 0))))))

(event Custom|StopFreeRoam
  (Variables|Default|SetFreeRoaming false))

(event EventTick
  (params (DeltaSeconds :type Float%20%28single-precision%29))
  (Variables|Default|SetDeltaT DeltaSeconds)
  (if (Variables|Default|GetFreeRoaming)
    (CallFunction|MovetoNextPoint)))

(fn ConstructionScript)